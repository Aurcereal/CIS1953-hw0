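; BP_EnemyBase is an enemy NPC Blueprint that relays AI perception changes to its AI controller.
; Each perception update flips SeesPlayer without inspecting what was sensed and prints the new value.
; After a short delay, it passes the flag to UpdateEnemyPerception on the BP_Enemy_AIController found by class lookup, rather than its own controller reference.
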(event `self.AIPerception.OnPerceptionUpdated`
  (params (UpdatedActors :type "Array of Actor Object Reference (by ref)"))
  (bind _seesplayer (`self.seesPlayer`))
  (set `self.seesPlayer` (not (`self.seesPlayer`)))
  (`KismetSystemLibrary.PrintString` (`KismetStringLibrary.Conv_BoolToString` _seesplayer))
  (bind _returnvalue (`GameplayStatics.GetActorOfClass` "/Game/NPC/BP_Enemy_AIController.BP_Enemy_AIController_C"))
  (`KismetSystemLibrary.Delay` 0.3)
  (`/Game/NPC/BP_Enemy_AIController.UpdateEnemyPerception` _returnvalue _seesplayer))

(fn `UserConstructionScript`
  (`parent.UserConstructionScript`))