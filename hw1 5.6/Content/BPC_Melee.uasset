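; BPC_Melee is a component that gives its owner a cooldown-limited melee attack against the first-person player character.
; TryAttack sphere-traces from the owner along the look direction returned by an interface message, with debug drawing left on.
; A hit on BP_FirstPersonCharacter removes one health through its BPCHealth component.
; Every permitted attempt, hit or miss, disables attacking until a timer fires AllowAttacking.
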(event `AllowAttacking`
  (set `self.CanAttack` true))

(event `TryAttack`
  (bind _returnvalue (`self.GetOwner`))
  (bind _returnvalue_2 (`Actor.K2_GetActorLocation` _returnvalue))
  (if (`self.CanAttack`)
    (bind _direction (message `/Game/BPCI_Character.GetLookDirection` _returnvalue))
    (bind _outhit (`KismetSystemLibrary.SphereTraceSingleForObjects` :`Start` _returnvalue_2 :`End` (+ (* _direction (`self.MeleeRange`)) _returnvalue_2) :`Radius` (`self.MeleeRadius`) :`ObjectTypes` (`|MakeArray` "ObjectTypeQuery2" "ObjectTypeQuery3" "ObjectTypeQuery4" :!type "EObjectTypeQuery Enum") :`DrawDebugType` "ForDuration" :`DrawTime` 0.15))
    (bind _asbp_first_person_character (cast `/Game/FirstPerson/Blueprints/BP_FirstPersonCharacter` (`.HitActor` (`GameplayStatics.BreakHitResult` _outhit)))
      (:`then`
        (`/Game/BPC_Health.ChangeHealth` (`/Game/FirstPerson/Blueprints/BP_FirstPersonCharacter.BPC_Health` _asbp_first_person_character) -1))
      (:`CastFailed`
        _))
    (set `self.CanAttack` false)
    (`KismetSystemLibrary.K2_SetTimerDelegate` (delegate `AllowAttacking`) (`self.Cooldown`))))