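; BP_Bullet is a projectile that reacts to hitting targets and first-person characters.
; On BeginPlay its Cone ignores IgnoreActor when moving, and that actor, if it casts to BPCI_Character, is told to ignore the bullet in return.
; On Hit it relocates a BP_Target randomly or takes one point from a BP_FirstPersonCharacter's health component.
; It destroys itself on any hit except against another bullet.
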(event `self.ReceiveBeginPlay`
  (bind _ignoreactor (`self.IgnoreActor`))
  (`PrimitiveComponent.IgnoreActorWhenMoving` (`self.Cone`) _ignoreactor true)
  (bind _asbpci_character (cast `/Game/BPCI_Character` _ignoreactor))
  (`/Game/BPCI_Character.IgnoreActorCollision` _asbpci_character self))

(event `self.ReceiveHit`
  (params (MyComp :type "PrimitiveComponent Object Reference") (Other :type "Actor Object Reference") (OtherComp :type "PrimitiveComponent Object Reference") (bSelfMoved :type Boolean) (HitLocation :type "Vector Structure") (HitNormal :type "Vector Structure") (NormalImpulse :type "Vector Structure") (Hit :type "HitResult Structure (by ref)"))
  (cast `/Game/BP_Bullet` Other
    (:`CastFailed`
      (bind _asbp_target (cast `/Game/BP_Target` Other)
        (:`then`
          (`/Game/BP_Target.RelocateRandomly` _asbp_target))
        (:`CastFailed`
          (bind _asbp_first_person_character (cast `/Game/FirstPerson/Blueprints/BP_FirstPersonCharacter` Other)
            (:`then`
              (`/Game/BPC_Health.ChangeHealth` (`/Game/FirstPerson/Blueprints/BP_FirstPersonCharacter.BPC_Health` _asbp_first_person_character) -1))
            (:`CastFailed`
              _))))
      (`self.K2_DestroyActor`))))

(fn `UserConstructionScript`)