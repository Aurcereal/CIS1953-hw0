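; BPC_Shoot is an actor component that lets its owner fire BP_Bullet projectiles from a limited, regenerating pool of charges.
; TryShoot spends a charge, spawns a bullet offset along the owner's look direction and launches it with an impulse on its Cone.
; Each shot restarts a timer for AddCharge, which re-arms itself until the charge cap is reached.
; The Awef function duplicates the shot logic without starting the recharge timer.
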(event `AddCharge`
  (set `self.Charges` (+ (`self.Charges`) 1))
  (if (< (`self.Charges`) 8)
    (`KismetSystemLibrary.K2_SetTimerDelegate` (delegate `AddCharge`) 2.0)))

(event `TryShoot`
  (bind _returnvalue (`self.GetOwner`))
  (if (> (`self.Charges`) 0)
    (set `self.Charges` (+ (`self.Charges`) -1))
    (`KismetSystemLibrary.K2_SetTimerDelegate` (delegate `AddCharge`) 2.0)
    (bind _direction (message `/Game/BPCI_Character.GetLookDirection` _returnvalue))
    (bind _returnvalue_2 (`|SpawnActorFromClass` "/Game/BP_Bullet.BP_Bullet_C" (`KismetMathLibrary.MakeTransform` (+ (* _direction (`self.Bullet Start Offset`)) (`Actor.K2_GetActorLocation` _returnvalue)) (`KismetMathLibrary.MakeRotFromZ` _direction)) "Undefined" "MultiplyWithRoot" null null))
    (`PrimitiveComponent.AddImpulse` (`/Game/BP_Bullet.Cone` _returnvalue_2) (* (`self.ImpulseStrength`) _direction) "None" false)))

(fn `awef`
  (bind _returnvalue (`self.GetOwner`))
  (if (> (`self.Charges`) 0)
    (set `self.Charges` (+ (`self.Charges`) -1))
    (bind _direction (message `/Game/BPCI_Character.GetLookDirection` _returnvalue))
    (bind _returnvalue_2 (`|SpawnActorFromClass` "/Game/BP_Bullet.BP_Bullet_C" (`KismetMathLibrary.MakeTransform` (+ (* _direction (`self.Bullet Start Offset`)) (`Actor.K2_GetActorLocation` _returnvalue)) (`KismetMathLibrary.MakeRotFromZ` _direction)) "Undefined" "MultiplyWithRoot" null null))
    (`PrimitiveComponent.AddImpulse` (`/Game/BP_Bullet.Cone` _returnvalue_2) (* (`self.ImpulseStrength`) _direction) "None" false)))