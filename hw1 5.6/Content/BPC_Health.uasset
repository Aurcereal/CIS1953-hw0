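; BPC_Health is a component that tracks the health of its owning actor and signals death.
; ChangeHealth adds a signed delta to Health without clamping, then sends OnDeathMessage to the owner whenever the result is zero or below.
; GetHealthFactor returns Health as a fraction of a hardcoded maximum rather than a variable.
; The component has no active BeginPlay or Tick logic.
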(fn `ChangeHealth`
  (params (Delta :type Integer))
  (bind _output_get (set `self.Health` (+ (`self.Health`) Delta)))
  (if (<= _output_get 0)
    (message `/Game/BPCI_Character.OnDeath` (`self.GetOwner`))))

(fn `GetHealthFactor`
  (returns (HealthFactor :type "Float (double-precision)"))
  (return (/ (`KismetMathLibrary.Conv_IntToDouble` (`self.Health`)) 8.0)))