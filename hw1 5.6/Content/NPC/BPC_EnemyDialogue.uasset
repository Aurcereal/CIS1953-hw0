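; Enemy dialogue component that stores a sequence of dialogue entries and tracks the current one by index.
; ProgressDialogue advances the index until the last entry and returns true if it moved, despite that flag being named IsLast.
; GetCurrentDialogue returns the entry at that index without a bounds check.
; The event graph is inactive, and ProgressDialogue retains an unconnected alternative version of its logic.
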(fn `GetCurrentDialogue`
  (returns (Dialogue :type String))
  (return (`|GetArrayItem` (`self.DialogueArray`) (`self.CurrentDialogue`))))

(fn `ProgressDialogue`
  (returns (HasNext :type Boolean))
  (locals (ReturningDialogue :type String) (IsLast :type Boolean :default true))
  (bind _islast (`local.IsLast`))
  (set `local.IsLast` (< (`self.CurrentDialogue`) (- (`KismetArrayLibrary.Array_Length` (`self.DialogueArray`)) 1)))
  (if _islast
    (set `self.CurrentDialogue` (+ (`self.CurrentDialogue`) 1)))
  (return _islast))