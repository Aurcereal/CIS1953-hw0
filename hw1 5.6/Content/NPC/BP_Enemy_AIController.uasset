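; BP_Enemy_AIController is the AI controller for enemy NPCs, linking them to the BT_Enemy_Base behavior tree.
; After a short delay on BeginPlay, it runs the tree and stores the first player pawn in the blackboard's player key.
; An UpdateEnemyPerception event switches the blackboard enemy state between two enum values depending on whether the player is seen.
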(event `self.ReceiveBeginPlay`
  (`KismetSystemLibrary.Delay` 0.2)
  (`self.RunBehaviorTree` "/Game/NPC/BT_Enemy_Base.BT_Enemy_Base")
  (`BlackboardComponent.SetValueAsObject` (`self.Blackboard`) (`self.PlayerKey`) (`GameplayStatics.GetPlayerPawn` 0)))

(event `UpdateEnemyPerception`
  (params (`Sees Player` :type Boolean))
  (`BlackboardComponent.SetValueAsEnum` (`self.Blackboard`) (`self.EnemyStateKey`) (select `bool` `Sees Player` :`false` (enumliteral `/Game/NPC/E_EnemyState` "NewEnumerator0") :`true` (enumliteral `/Game/NPC/E_EnemyState` "NewEnumerator3"))))

(fn `UserConstructionScript`)